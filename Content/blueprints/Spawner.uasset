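; Spawner actor that periodically creates BP_Geometry actors at random locations among its spawn points.
; On BeginPlay it starts a looping timer, with its interval set by SpawnSpeed, that calls SpawnGeometry.
; Each call picks one of seven spawn point transforms at random and spawns a BP_Geometry there.
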(event `self.ReceiveBeginPlay`
  (`KismetSystemLibrary.K2_SetTimer` null "SpawnGeometry" (`self.SpawnSpeed`) true))

(fn `SpawnGeometry`
  (`|SpawnActorFromClass` "/Game/blueprints/Geometry/BP_Geometry.BP_Geometry_C" (`|GetArrayItem` (`|MakeArray` (`SceneComponent.K2_GetComponentToWorld` (`self.SpawnPoint1`)) (`SceneComponent.K2_GetComponentToWorld` (`self.SpawnPoint2`)) (`SceneComponent.K2_GetComponentToWorld` (`self.SpawnPoint3`)) (`SceneComponent.K2_GetComponentToWorld` (`self.SpawnPoint4`)) (`SceneComponent.K2_GetComponentToWorld` (`self.SpawnPoint5`)) (`SceneComponent.K2_GetComponentToWorld` (`self.SpawnPoint6`)) (`SceneComponent.K2_GetComponentToWorld` (`self.SpawnPoint`))) (`KismetMathLibrary.RandomIntegerInRange` 0 6)) "Undefined" "OverrideRootScale" null null))

(fn `UserConstructionScript`)