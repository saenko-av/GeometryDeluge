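; Player pawn for a shape-catching game that moves on the Moveright axis along GeometryL's forward vector.
; BeginPlay gives GeometryL a random box, circle, cross or triangle mesh.
; Left-box overlaps with matching BP_Geometry increment savGameMode's Catched count and destroy the actor; mismatches decrement it when positive.
; Second-to-fourth shape generators all target GeometryR but never run, leaving the right side unused.
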(event `InputAxis|Moveright`
  (params (AxisValue :type "Float (single-precision)"))
  (`self.AddMovementInput` (`SceneComponent.GetForwardVector` (`self.geometryL`)) (* (`self.MoveSpeed`) AxisValue)))

(event `self.ReceiveBeginPlay`
  (`self.GenerateFirstPlayer`))

(event `self.CollisionBoxL.OnComponentBeginOverlap`
  (params (OverlappedComponent :type "PrimitiveComponent Object Reference") (OtherActor :type "Actor Object Reference") (OtherComp :type "PrimitiveComponent Object Reference") (OtherBodyIndex :type Integer) (bFromSweep :type Boolean) (SweepResult :type "HitResult Structure (by ref)"))
  (bind _asbp_geometry (cast `/Game/blueprints/Geometry/BP_Geometry` OtherActor))
  (if (== (`/Game/blueprints/Geometry/BP_Geometry.GeometryName` _asbp_geometry) (`self.FirstActiveStaticMesh`))
    (bind _assav_game_mode (cast `/Game/blueprints/Engine/savGameMode` (`GameplayStatics.GetGameMode`)))
    (`/Engine/EditorBlueprintResources/StandardMacros.IncrementInt` (`/Game/blueprints/Engine/savGameMode.Catched` _assav_game_mode)
      (:`  `
        (`self.K2_DestroyActor` _asbp_geometry)))
    (else
      (bind _assav_game_mode_2 (cast `/Game/blueprints/Engine/savGameMode` (`GameplayStatics.GetGameMode`)))
      (bind _catched (`/Game/blueprints/Engine/savGameMode.Catched` _assav_game_mode_2))
      (if (> (`KismetMathLibrary.Conv_IntToByte` _catched) 0)
        (`/Engine/EditorBlueprintResources/StandardMacros.DecrementInt` _catched)))))

(fn `GenerateFirstPlayer`
  (bind _output_get (set `self.FirstActiveStaticMesh` (`|GetArrayItem` (`|MakeArray` (`self.box`) (`self.circle`) (`self.cross`) (`self.triangle`)) (`KismetMathLibrary.RandomIntegerInRange` 0 3))))
  (`StaticMeshComponent.SetStaticMesh` (`self.geometryL`) _output_get))

(fn `GenerateFourthPlayer`
  (bind _output (`|GetArrayItem` (`|MakeArray` (`self.box`) (`self.circle`) (`self.cross`) (`self.triangle`)) (`KismetMathLibrary.RandomIntegerInRange` 0 3)))
  (while (and (!= _output (`self.FirstActiveStaticMesh`)) (and (!= _output (`self.SecondActiveStaticMesh`)) (!= _output (`self.ThirdActiveStaticMesh`))))
    (bind _output_get (set `self.SecondActiveStaticMesh` _output))
    (`StaticMeshComponent.SetStaticMesh` (`self.geometryR`) _output_get)))

(fn `GenerateSecondPlayer`
  (bind _output (`|GetArrayItem` (`|MakeArray` (`self.box`) (`self.circle`) (`self.cross`) (`self.triangle`)) (`KismetMathLibrary.RandomIntegerInRange` 0 3)))
  (while (!= _output (`self.FirstActiveStaticMesh`))
    (bind _output_get (set `self.SecondActiveStaticMesh` _output))
    (`StaticMeshComponent.SetStaticMesh` (`self.geometryR`) _output_get)))

(fn `GenerateThirdPlayer`
  (bind _output (`|GetArrayItem` (`|MakeArray` (`self.box`) (`self.circle`) (`self.cross`) (`self.triangle`)) (`KismetMathLibrary.RandomIntegerInRange` 0 3)))
  (while (and (!= _output (`self.FirstActiveStaticMesh`)) (!= _output (`self.SecondActiveStaticMesh`)))
    (bind _output_get (set `self.SecondActiveStaticMesh` _output))
    (`StaticMeshComponent.SetStaticMesh` (`self.geometryR`) _output_get)))

(fn `UserConstructionScript`)