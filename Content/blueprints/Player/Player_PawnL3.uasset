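; Player pawn for a shape-catching game that shows a random box, circle, cross or triangle mesh on BeginPlay.
; Touch input eases CollisionBoxL toward the screen-centered X position, while the Moveright axis adds movement input along the mesh's forward vector.
; Overlapping a matching BP_GeometryL1 increments the savGameInstance Catched count and destroys it; a mismatch decrements the count if above zero.
; Generators for second through fourth shapes contain only unreachable logic.
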(event `InputTouch`
  (params (Location :type "Vector Structure") (FingerIndex :type "ETouchIndex Enum"))
  (bind _returnvalue_x (`KismetMathLibrary.BreakVector2D` (`WidgetLayoutLibrary.GetViewportSize`)))
  ;[1 1 1] InputTouch Move
  (:`Pressed`
    (`KismetSystemLibrary.MoveComponentTo` (`self.CollisionBoxL`) (`KismetMathLibrary.MakeVector` (- (.x Location) (/ _returnvalue_x 2.0))) (struct) true true 0.05 :!label _label))
  (:`Released`
    (goto _label :!via `Stop`))
  (:`Moved`
    (goto _label)))

(event `InputAxis|Moveright`
  (params (AxisValue :type "Float (single-precision)"))
  (`self.AddMovementInput` (`SceneComponent.GetForwardVector` (`self.geometryL`)) (* (`self.MoveSpeed`) AxisValue)))

(event `self.ReceiveBeginPlay`
  (`self.GenerateFirstPlayer`))

(event `self.CollisionBoxL.OnComponentBeginOverlap`
  (params (OverlappedComponent :type "PrimitiveComponent Object Reference") (OtherActor :type "Actor Object Reference") (OtherComp :type "PrimitiveComponent Object Reference") (OtherBodyIndex :type Integer) (bFromSweep :type Boolean) (SweepResult :type "HitResult Structure (by ref)"))
  (bind _asbp_geometry_l1 (cast `/Game/blueprints/Geometry/BP_GeometryL1` OtherActor))
  (if (== (`/Game/blueprints/Geometry/BP_GeometryL1.GeometryName` _asbp_geometry_l1) (`self.FirstActiveStaticMesh`))
    (bind _assav_game_instance (cast `/Game/blueprints/Engine/savGameInstance` (`GameplayStatics.GetGameInstance`)))
    (`/Engine/EditorBlueprintResources/StandardMacros.IncrementInt` (`/Game/blueprints/Engine/savGameInstance.Catched` _assav_game_instance)
      (:`  `
        (`self.K2_DestroyActor` _asbp_geometry_l1)))
    (else
      (bind _assav_game_instance_2 (cast `/Game/blueprints/Engine/savGameInstance` (`GameplayStatics.GetGameInstance`)))
      (bind _catched (`/Game/blueprints/Engine/savGameInstance.Catched` _assav_game_instance_2))
      (if (> (`KismetMathLibrary.Conv_IntToByte` _catched) 0)
        (`/Engine/EditorBlueprintResources/StandardMacros.DecrementInt` _catched)))))

(fn `GenerateFirstPlayer`
  (bind _output_get (set `self.FirstActiveStaticMesh` (`|GetArrayItem` (`|MakeArray` (`self.box`) (`self.circle`) (`self.cross`) (`self.triangle`)) (`KismetMathLibrary.RandomIntegerInRange` 0 3))))
  (`StaticMeshComponent.SetStaticMesh` (`self.geometryL`) _output_get))

(fn `GenerateFourthPlayer`)

(fn `GenerateSecondPlayer`)

(fn `GenerateThirdPlayer`)

(fn `UserConstructionScript`)