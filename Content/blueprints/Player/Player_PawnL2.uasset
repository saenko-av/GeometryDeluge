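; Level 2 player pawn that moves on the Moveright axis and catches falling or placed BP_GeometryL2 shapes matching its own geometry.
; BeginPlay randomly assigns meshes to GeometryL and GeometryL1, each assignment overwriting the PanwL2Geometry match array.
; CollisionBoxL overlaps compare arrays: matches increment savGameInstance's Catched and destroy the shape, while mismatches decrement it above zero.
; Third and fourth player generators are empty, with unconnected draft logic.
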(event `InputAxis|Moveright`
  (params (AxisValue :type "Float (single-precision)"))
  (`self.AddMovementInput` (`SceneComponent.GetForwardVector` (`self.geometryL`)) (* (`self.MoveSpeed`) AxisValue)))

(event `self.ReceiveBeginPlay`
  (`self.GenerateFirstPlayer`)
  (`self.GenerateSecondPlayer`))

(event `self.CollisionBoxL.OnComponentBeginOverlap`
  (params (OverlappedComponent :type "PrimitiveComponent Object Reference") (OtherActor :type "Actor Object Reference") (OtherComp :type "PrimitiveComponent Object Reference") (OtherBodyIndex :type Integer) (bFromSweep :type Boolean) (SweepResult :type "HitResult Structure (by ref)"))
  (bind _asbp_geometry_l2 (cast `/Game/blueprints/Geometry/BP_GeometryL2` OtherActor))
  (if (`KismetArrayLibrary.Array_Identical` (`/Game/blueprints/Geometry/BP_GeometryL2.GeometryL2Mesh` _asbp_geometry_l2) (`self.PanwL2Geometry`))
    (bind _assav_game_instance (cast `/Game/blueprints/Engine/savGameInstance` (`GameplayStatics.GetGameInstance`)))
    (`/Engine/EditorBlueprintResources/StandardMacros.IncrementInt` (`/Game/blueprints/Engine/savGameInstance.Catched` _assav_game_instance)
      (:`  `
        (`self.K2_DestroyActor` _asbp_geometry_l2)))
    (else
      (bind _assav_game_instance_2 (cast `/Game/blueprints/Engine/savGameInstance` (`GameplayStatics.GetGameInstance`)))
      (bind _catched (`/Game/blueprints/Engine/savGameInstance.Catched` _assav_game_instance_2))
      (if (> (`KismetMathLibrary.Conv_IntToByte` _catched) 0)
        (`/Engine/EditorBlueprintResources/StandardMacros.DecrementInt` _catched)))))

(fn `GenerateFirstPlayer`
  (bind _output_get (set `self.FirstActiveStaticMesh` (`|GetArrayItem` (`|MakeArray` (`self.box`) (`self.circle`) (`self.cross`) (`self.triangle`)) (`KismetMathLibrary.RandomIntegerInRange` 0 3))))
  (`StaticMeshComponent.SetStaticMesh` (`self.geometryL`) _output_get)
  (set `self.PanwL2Geometry` (`|MakeArray` _output_get)))

(fn `GenerateFourthPlayer`)

(fn `GenerateSecondPlayer`
  (bind _output (`|GetArrayItem` (`|MakeArray` (`self.box`) (`self.circle`) (`self.cross`) (`self.triangle`)) (`KismetMathLibrary.RandomIntegerInRange` 0 3)))
  (while (!= _output (`self.FirstActiveStaticMesh`))
    (bind _output_get (set `self.SecondActiveStaticMesh` _output))
    (`StaticMeshComponent.SetStaticMesh` (`self.geometryL1`) _output_get)
    (set `self.PanwL2Geometry` (`|MakeArray` _output_get))))

(fn `GenerateThirdPlayer`)

(fn `UserConstructionScript`)