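; Player pawn, apparently for a survival mode, that the player steers along one axis by dragging a finger on the touchscreen.
; Touch movement converts the finger's X offset from the viewport center into a scaled relative X location for the collision box, applied with sweep.
; On BeginPlay, GeneratePlayer gives the pawn a random shape mesh from a small fixed set.
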(event `InputTouch`
  (params (Location :type "Vector Structure") (FingerIndex :type "ETouchIndex Enum"))
  (bind _returnvalue_x (`KismetMathLibrary.BreakVector2D` (`WidgetLayoutLibrary.GetViewportSize`)))
  ;[1 1 1] InputTouch Move
  (:`Moved`
    (`SceneComponent.K2_SetRelativeLocation` (`self.CollisionBoxL`) (`KismetMathLibrary.MakeVector` (* (- (.x Location) (/ _returnvalue_x 2.0)) 1.5)) true false)))

(event `self.ReceiveBeginPlay`
  (`self.GeneratePlayer`))

(fn `GeneratePlayer`
  (bind _output_get (set `self.ActiveStaticMesh` (`|GetArrayItem` (`|MakeArray` (`self.box`) (`self.circle`) (`self.cross`) (`self.triangle`)) (`KismetMathLibrary.RandomIntegerInRange` 0 3))))
  (`StaticMeshComponent.SetStaticMesh` (`self.geometryL`) _output_get))

(fn `UserConstructionScript`)