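; Player pawn for a shape-matching catch game: it takes a random mesh (box, circle, cross or triangle) on BeginPlay.
; Touch moves set a target X offset from SLocation, applied and debug-printed every Tick; a Moveright axis also adds movement input.
; Overlapping matching BP_GeometryL1 actors raises Catched and destroys them; mismatches drain Catched, then Health, then pause the game.
; Screen-half steering and second-to-fourth shape generators are unwired.
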(event `InputTouch`
  (params (Location :type "Vector Structure") (FingerIndex :type "ETouchIndex Enum"))
  (:`Moved`
    (set `self.ELocation` (+ (`self.SLocation`) (`KismetMathLibrary.MakeVector` (`PlayerController.GetInputTouchState` (`GameplayStatics.GetPlayerController` 0) "Touch1"))))))

(event `self.ReceiveTick`
  (params (DeltaSeconds :type "Float (single-precision)"))
  (`self.K2_SetActorLocation` (`self.ELocation`))
  (`KismetSystemLibrary.PrintString` (`KismetStringLibrary.Conv_VectorToString` (`KismetMathLibrary.MakeVector` (`PlayerController.GetInputTouchState` (`GameplayStatics.GetPlayerController` 0) "Touch1")))))

(event `InputTouch`
  (params (Location :type "Vector Structure") (FingerIndex :type "ETouchIndex Enum"))
  ;[1 1 1] Tap on Left/Right part of screen to move here
)

(event `InputAxis|Moveright`
  (params (AxisValue :type "Float (single-precision)"))
  ;[1 1 1] Touch Movemment
  (`self.AddMovementInput` (`SceneComponent.GetForwardVector` (`self.geometryL`)) (* (`self.MoveSpeed`) AxisValue)))

(event `self.ReceiveBeginPlay`
  (`self.GenerateFirstPlayer`))

(event `self.CollisionBoxL.OnComponentBeginOverlap`
  (params (OverlappedComponent :type "PrimitiveComponent Object Reference") (OtherActor :type "Actor Object Reference") (OtherComp :type "PrimitiveComponent Object Reference") (OtherBodyIndex :type Integer) (bFromSweep :type Boolean) (SweepResult :type "HitResult Structure (by ref)"))
  (bind _asbp_geometry_l1 (cast `/Game/blueprints/Geometry/BP_GeometryL1` OtherActor))
  (if (== (`/Game/blueprints/Geometry/BP_GeometryL1.GeometryName` _asbp_geometry_l1) (`self.FirstActiveStaticMesh`))
    (bind _assav_game_instance (cast `/Game/blueprints/Engine/savGameInstance` (`GameplayStatics.GetGameInstance`)))
    (`/Engine/EditorBlueprintResources/StandardMacros.IncrementInt` (`/Game/blueprints/Engine/savGameInstance.Catched` _assav_game_instance)
      (:`  `
        (`self.K2_DestroyActor` _asbp_geometry_l1)))
    (else
      (bind _assav_game_instance_2 (cast `/Game/blueprints/Engine/savGameInstance` (`GameplayStatics.GetGameInstance`)))
      (bind _catched (`/Game/blueprints/Engine/savGameInstance.Catched` _assav_game_instance_2))
      (if (> (`KismetMathLibrary.Conv_IntToByte` _catched) 0)
        (`/Engine/EditorBlueprintResources/StandardMacros.DecrementInt` _catched)
        (else
          (bind _assav_game_instance_3 (cast `/Game/blueprints/Engine/savGameInstance` (`GameplayStatics.GetGameInstance`)))
          (bind _health (`/Game/blueprints/Engine/savGameInstance.Health` _assav_game_instance_3))
          (if (>= _health 0)
            (`/Engine/EditorBlueprintResources/StandardMacros.DecrementInt` _health)
            (else
              (`GameplayStatics.SetGamePaused` true))))))))

(fn `GenerateFirstPlayer`
  (bind _output_get (set `self.FirstActiveStaticMesh` (`|GetArrayItem` (`|MakeArray` (`self.box`) (`self.circle`) (`self.cross`) (`self.triangle`)) (`KismetMathLibrary.RandomIntegerInRange` 0 3))))
  (`StaticMeshComponent.SetStaticMesh` (`self.geometryL`) _output_get))

(fn `GenerateFourthPlayer`)

(fn `GenerateSecondPlayer`)

(fn `GenerateThirdPlayer`)

(fn `UserConstructionScript`)