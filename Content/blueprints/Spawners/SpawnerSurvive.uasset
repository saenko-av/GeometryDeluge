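; Spawner actor that can place BP_Survive actors at one of eight spawn point components picked at random.
; Tick lowers DelayDuration by elapsed game time divided by 100 each frame and prints it, with no lower limit.
; The SpawnWaveSpead timeline's update would delay by that value and call SpawnGeometry, but this chain never runs, so the file itself triggers no spawns.
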(event `self.ReceiveTick`
  (params (DeltaSeconds :type "Float (single-precision)"))
  ;[1 1 1] From Catchet to Wave speed
  (bind _output_get (set `self.Delay Duration` (- (`self.Delay Duration`) (/ (`KismetSystemLibrary.GetGameTimeInSeconds`) 100.0))))
  (`KismetSystemLibrary.PrintString` (`KismetStringLibrary.Conv_DoubleToString` _output_get)))

(fn `SpawnGeometry`
  (`|SpawnActorFromClass` "/Game/blueprints/Geometry/BP_Survive.BP_Survive_C" (`|GetArrayItem` (`|MakeArray` (`SceneComponent.K2_GetComponentToWorld` (`self.SpawnPoint1`)) (`SceneComponent.K2_GetComponentToWorld` (`self.SpawnPoint2`)) (`SceneComponent.K2_GetComponentToWorld` (`self.SpawnPoint3`)) (`SceneComponent.K2_GetComponentToWorld` (`self.SpawnPoint4`)) (`SceneComponent.K2_GetComponentToWorld` (`self.SpawnPoint5`)) (`SceneComponent.K2_GetComponentToWorld` (`self.SpawnPoint6`)) (`SceneComponent.K2_GetComponentToWorld` (`self.SpawnPoint`)) (`SceneComponent.K2_GetComponentToWorld` (`self.SpawnPoint7`))) (`KismetMathLibrary.RandomIntegerInRange` 0 7)) "Undefined" "OverrideRootScale" null null))

(fn `UserConstructionScript`)