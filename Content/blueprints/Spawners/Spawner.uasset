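; Spawner actor that drops BP_Geometry, or a rare BPLife pickup, at one of seven random spawn points.
; Tick shortens the spawn delay as the saved Catched count rises, with a one-shot drop at a threshold that the next tick recalculates.
; The SpawnWaveSpead timeline's Update waits that delay before calling SpawnGeometry, though no wire in the graph starts the timeline.
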(event `self.ReceiveTick`
  (params (DeltaSeconds :type "Float (single-precision)"))
  ;[1 1 1] From Catchet to Wave speed
  (bind _assav_game_instance (cast `/Game/blueprints/Engine/savGameInstance` (`GameplayStatics.GetGameInstance`)))
  (bind _returnvalue (`KismetMathLibrary.Conv_IntToDouble` (`/Game/blueprints/Engine/savGameInstance.Catched` _assav_game_instance)))
  (bind _output_get (set `self.Delay Duration` (- (`self.SpawnSpeed`) (/ _returnvalue 100.0))))
  ;[1 1 1] New Level
  (if (>= _returnvalue 90.0)
    (`/Engine/EditorBlueprintResources/StandardMacros.DoOnce` false
      (:`Completed`
        (set `self.Delay Duration` 0.1)))))

(fn `SpawnGeometry`
  (bind _output (`|GetArrayItem` (`|MakeArray` (`SceneComponent.K2_GetComponentToWorld` (`self.SpawnPoint1`)) (`SceneComponent.K2_GetComponentToWorld` (`self.SpawnPoint2`)) (`SceneComponent.K2_GetComponentToWorld` (`self.SpawnPoint3`)) (`SceneComponent.K2_GetComponentToWorld` (`self.SpawnPoint4`)) (`SceneComponent.K2_GetComponentToWorld` (`self.SpawnPoint5`)) (`SceneComponent.K2_GetComponentToWorld` (`self.SpawnPoint6`)) (`SceneComponent.K2_GetComponentToWorld` (`self.SpawnPoint`))) (`KismetMathLibrary.RandomIntegerInRange` 0 6)))
  (if (`KismetMathLibrary.InRange_FloatFloat` (`KismetMathLibrary.RandomFloatInRange` 0.0 1.0) 0.0 0.05)
    (`|SpawnActorFromClass` (`|GetArrayItem` (`|MakeArray` (`self.BP Life`))) _output "Undefined" "OverrideRootScale" null null)
    (else
      (`|SpawnActorFromClass` "/Game/blueprints/Geometry/BP_Geometry.BP_Geometry_C" _output "Undefined" "OverrideRootScale" null null))))

(fn `UserConstructionScript`)