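; Level 5 spawner actor that defines random geometry spawns and scales their delay with the player's catch count.
; Tick shortens the delay as the savGameMode catch count rises and prints "New Level" once it reaches three.
; SpawnGeometry picks among seven points for BP_GeometryL1; SpawnGeometryReverseble picks among fourteen for BP_GeometryL5.
; The delayed timeline spawn loop never runs, and nothing here calls the reversible variant.
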(event `self.ReceiveTick`
  (params (DeltaSeconds :type "Float (single-precision)"))
  ;[1 1 1] From Catchet to Wave speed
  (bind _assav_game_mode (cast `/Game/blueprints/Engine/savGameMode` (`GameplayStatics.GetGameMode`)))
  (bind _returnvalue (`KismetMathLibrary.Conv_IntToDouble` (`/Game/blueprints/Engine/savGameMode.Catched` _assav_game_mode)))
  (bind _output_get (set `self.Delay Duration` (- (`self.SpawnSpeed`) (/ _returnvalue 30.0))))
  ;[1 1 1] New Level
  (if (>= _returnvalue 3.0)
    (`/Engine/EditorBlueprintResources/StandardMacros.DoOnce` false :!label _label
      (:`Completed`
        (`KismetSystemLibrary.PrintString` "New Level")))
    (else
      (goto _label :!via `Reset`))))

(fn `SpawnGeometry`
  (`|SpawnActorFromClass` "/Game/blueprints/Geometry/BP_GeometryL1.BP_GeometryL1_C" (`|GetArrayItem` (`|MakeArray` (`SceneComponent.K2_GetComponentToWorld` (`self.SpawnPoint1`)) (`SceneComponent.K2_GetComponentToWorld` (`self.SpawnPoint2`)) (`SceneComponent.K2_GetComponentToWorld` (`self.SpawnPoint3`)) (`SceneComponent.K2_GetComponentToWorld` (`self.SpawnPoint4`)) (`SceneComponent.K2_GetComponentToWorld` (`self.SpawnPoint5`)) (`SceneComponent.K2_GetComponentToWorld` (`self.SpawnPoint6`)) (`SceneComponent.K2_GetComponentToWorld` (`self.SpawnPoint`))) (`KismetMathLibrary.RandomIntegerInRange` 0 6)) "Undefined" "OverrideRootScale" null null))

(fn `SpawnGeometryReverseble`
  (`|SpawnActorFromClass` "/Game/blueprints/Geometry/BP_GeometryL5.BP_GeometryL5_C" (`|GetArrayItem` (`|MakeArray` (`SceneComponent.K2_GetComponentToWorld` (`self.SpawnPoint1`)) (`SceneComponent.K2_GetComponentToWorld` (`self.SpawnPoint2`)) (`SceneComponent.K2_GetComponentToWorld` (`self.SpawnPoint3`)) (`SceneComponent.K2_GetComponentToWorld` (`self.SpawnPoint4`)) (`SceneComponent.K2_GetComponentToWorld` (`self.SpawnPoint5`)) (`SceneComponent.K2_GetComponentToWorld` (`self.SpawnPoint6`)) (`SceneComponent.K2_GetComponentToWorld` (`self.SpawnPoint`)) (`SceneComponent.K2_GetComponentToWorld` (`self.SpawnPoint8`)) (`SceneComponent.K2_GetComponentToWorld` (`self.SpawnPoint9`)) (`SceneComponent.K2_GetComponentToWorld` (`self.SpawnPoint10`)) (`SceneComponent.K2_GetComponentToWorld` (`self.SpawnPoint11`)) (`SceneComponent.K2_GetComponentToWorld` (`self.SpawnPoint12`)) (`SceneComponent.K2_GetComponentToWorld` (`self.SpawnPoint13`)) (`SceneComponent.K2_GetComponentToWorld` (`self.SpawnPoint7`))) (`KismetMathLibrary.RandomIntegerInRange` 0 13)) "Undefined" "OverrideRootScale" null null))

(fn `UserConstructionScript`)