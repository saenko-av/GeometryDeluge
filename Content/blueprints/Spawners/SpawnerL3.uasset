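; Level 3 spawner that places BP_GeometryL3 actors at one of seven spawn points, picked at random.
; Tick shortens the spawn delay as the saved game instance's Catched count rises, and prints a one-time "New Level" message at a threshold, re-armed below it.
; The SpawnWaveSpead update chain waits that delay before calling SpawnGeometry, though nothing in the graph starts it.
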(event `self.ReceiveTick`
  (params (DeltaSeconds :type "Float (single-precision)"))
  ;[1 1 1] From Catchet to Wave speed
  (bind _assav_game_instance (cast `/Game/blueprints/Engine/savGameInstance` (`GameplayStatics.GetGameInstance`)))
  (bind _returnvalue (`KismetMathLibrary.Conv_IntToDouble` (`/Game/blueprints/Engine/savGameInstance.Catched` _assav_game_instance)))
  (bind _output_get (set `self.Delay Duration` (- (`self.SpawnSpeed`) (/ _returnvalue 30.0))))
  ;[1 1 1] New Level
  (if (>= _returnvalue 3.0)
    (`/Engine/EditorBlueprintResources/StandardMacros.DoOnce` false :!label _label
      (:`Completed`
        (`KismetSystemLibrary.PrintString` "New Level")))
    (else
      (goto _label :!via `Reset`))))

(fn `SpawnGeometry`
  (`|SpawnActorFromClass` "/Game/blueprints/Geometry/BP_GeometryL3.BP_GeometryL3_C" (`|GetArrayItem` (`|MakeArray` (`SceneComponent.K2_GetComponentToWorld` (`self.SpawnPoint1`)) (`SceneComponent.K2_GetComponentToWorld` (`self.SpawnPoint2`)) (`SceneComponent.K2_GetComponentToWorld` (`self.SpawnPoint3`)) (`SceneComponent.K2_GetComponentToWorld` (`self.SpawnPoint4`)) (`SceneComponent.K2_GetComponentToWorld` (`self.SpawnPoint5`)) (`SceneComponent.K2_GetComponentToWorld` (`self.SpawnPoint6`)) (`SceneComponent.K2_GetComponentToWorld` (`self.SpawnPoint`))) (`KismetMathLibrary.RandomIntegerInRange` 0 6)) "Undefined" "OverrideRootScale" null null))

(fn `UserConstructionScript`)