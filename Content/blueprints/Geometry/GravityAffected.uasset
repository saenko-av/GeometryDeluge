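; Actor whose Cube is pulled toward the player's Survive_Pawn, acting as an object affected by player-centred gravity.
; Each tick it finds the look-at direction from the Cube to the pawn and adds that direction, scaled by Gravity, to the Cube's physics linear velocity.
; The pull does not vary with distance, as the distance calculation is left unconnected, and is not scaled by delta time.
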(event `self.ReceiveTick`
  (params (DeltaSeconds :type "Float (single-precision)"))
  (bind _assurvive_pawn (cast `/Game/blueprints/Player/Survive_Pawn` (`GameplayStatics.GetPlayerPawn` 0)))
  (`PrimitiveComponent.SetPhysicsLinearVelocity` (`self.Cube`) (* (`KismetMathLibrary.GetForwardVector` (`KismetMathLibrary.FindLookAtRotation` (`SceneComponent.K2_GetComponentLocation` (`self.Cube`)) (`SceneComponent.K2_GetComponentLocation` (`Actor.RootComponent` _assurvive_pawn)))) (`self.Gravity`)) true "None"))

(fn `UserConstructionScript`)