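; Geometry Survive actor that randomly assigns Box, Cross, Triangle or Circle meshes to its three static mesh components on BeginPlay.
; The first mesh is a single random pick, which the second and third generators compare against in while loops, with the third also checking the second.
; Each loop check and assignment rolls separately, so distinct shapes are not guaranteed and the second or third mesh may never be set.
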(event `self.ReceiveBeginPlay`
  (`self.GenerateFirstStaticMesh`)
  (`self.GenerateSecondStaticMesh`)
  (`self.GenerateThirdStaticMesh`))

(fn `GenerateFirstStaticMesh`
  (bind _output_get (set `self.FirstStaticMesh` (`|GetArrayItem` (`|MakeArray` (`self.box`) (`self.cross`) (`self.triangle`) (`self.circle`)) (`KismetMathLibrary.RandomIntegerInRange` 0 3))))
  (`StaticMeshComponent.SetStaticMesh` (`self.FirsStatic`) _output_get))

(fn `GenerateSecondStaticMesh`
  (bind _output (`|GetArrayItem` (`|MakeArray` (`self.box`) (`self.circle`) (`self.cross`) (`self.triangle`)) (`KismetMathLibrary.RandomIntegerInRange` 0 3)))
  (while (!= _output (`self.FirstStaticMesh`))
    (bind _output_get (set `self.SecondStaticMesh` _output))
    (`StaticMeshComponent.SetStaticMesh` (`self.SecondStatic`) _output_get)))

(fn `GenerateThirdStaticMesh`
  (bind _output (`|GetArrayItem` (`|MakeArray` (`self.box`) (`self.circle`) (`self.cross`) (`self.triangle`)) (`KismetMathLibrary.RandomIntegerInRange` 0 3)))
  (while (and (!= _output (`self.FirstStaticMesh`)) (!= _output (`self.SecondStaticMesh`)))
    (bind _output_get (set `self.ThirdStaticMesh` _output))
    (`StaticMeshComponent.SetStaticMesh` (`self.ThirdStatic`) _output_get)))

(fn `UserConstructionScript`)