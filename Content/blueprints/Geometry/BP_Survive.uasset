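; BP_Survive is a randomized geometry actor that is pulled toward the player's Survive_Pawn.
; On BeginPlay it picks one of four shape meshes, a uniform scale within a range and one of three colored materials for SpawnGeometry.
; Each Tick it adds linear velocity toward the pawn, scaled by Gravity, so the pull accumulates per frame without delta-time or distance scaling.
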(event `self.ReceiveBeginPlay`
  (bind _output_get (set `self.GeometryName` (`|GetArrayItem` (`|MakeArray` (`self.box`) (`self.cross`) (`self.triangle`) (`self.circle`)) (`KismetMathLibrary.RandomIntegerInRange` 0 3))))
  (`StaticMeshComponent.SetStaticMesh` (`self.SpawnGeometry`) _output_get)
  (bind _output_get_2 (set `self.Scale` (`KismetMathLibrary.RandomFloatInRange` 0.5 1.5)))
  (`SceneComponent.SetRelativeScale3D` (`self.SpawnGeometry`) (`KismetMathLibrary.Conv_DoubleToVector` _output_get_2))
  (bind _output_get_3 (set `self.NewMaterial` (`|GetArrayItem` (`|MakeArray` (`self.BlueMI`) (`self.RedMI`) (`self.YellowMI`)) (`KismetMathLibrary.RandomIntegerInRange` 0 2))))
  (`PrimitiveComponent.SetMaterial` (`self.SpawnGeometry`) 0 _output_get_3))

(event `self.ReceiveTick`
  (params (DeltaSeconds :type "Float (single-precision)"))
  (bind _assurvive_pawn (cast `/Game/blueprints/Player/Survive_Pawn` (`GameplayStatics.GetPlayerPawn` 0)))
  (`PrimitiveComponent.SetPhysicsLinearVelocity` (`self.SpawnGeometry`) (* (`KismetMathLibrary.GetForwardVector` (`KismetMathLibrary.FindLookAtRotation` (`SceneComponent.K2_GetComponentLocation` (`self.SpawnGeometry`)) (`SceneComponent.K2_GetComponentLocation` (`Actor.RootComponent` _assurvive_pawn)))) (`self.Gravity`)) true "None"))

(fn `UserConstructionScript`)