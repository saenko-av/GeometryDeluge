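; BP_GeometryL2 is a geometry Blueprint that shows random shapes (box, cross, triangle or circle) on two static mesh components at BeginPlay.
; The first pick is stored and compared against in a while loop that re-rolls the second until a random test roll matches the first.
; The assigned second shape is rolled separately, so it can duplicate the first or stay unset.
; GeometryL2Mesh is overwritten with the latest single mesh; the two-mesh assignment is unconnected.
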(event `self.ReceiveBeginPlay`
  (`self.GenerateFirstStaticMesh`)
  (`self.GenerateSecondStaticMesh`))

(fn `GenerateFirstStaticMesh`
  (bind _output_get (set `self.FirstActiveStaticMesh` (`|GetArrayItem` (`|MakeArray` (`self.box`) (`self.cross`) (`self.triangle`) (`self.circle`)) (`KismetMathLibrary.RandomIntegerInRange` 0 3))))
  (`StaticMeshComponent.SetStaticMesh` (`self.FirstStaticMesh`) _output_get)
  (set `self.GeometryL2Mesh` (`|MakeArray` _output_get)))

(fn `GenerateSecondStaticMesh`
  (bind _output (`|GetArrayItem` (`|MakeArray` (`self.box`) (`self.circle`) (`self.cross`) (`self.triangle`)) (`KismetMathLibrary.RandomIntegerInRange` 0 3)))
  (while (!= _output (`self.FirstActiveStaticMesh`))
    (bind _output_get (set `self.SecondActiveStaticMesh` _output))
    (`StaticMeshComponent.SetStaticMesh` (`self.SecondStaticMesh`) _output_get)
    (set `self.GeometryL2Mesh` (`|MakeArray` _output_get))))

(fn `UserConstructionScript`)